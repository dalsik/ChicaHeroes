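; BP_Glitch drives a screen glitch post-process effect, with Glitch, HitGlitch and GlitchOut events as variants.
; Each event creates a new dynamic instance of M_GlitchEffect, adds it to the PostProcess component as a blendable, then plays its own timeline to animate GlitchStrength.
; HitGlitch also starts a red camera fade on the first player's camera as hit feedback.
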(event Custom|GlitchOut
  ;[0.15 0.15 0.15 0.5] GlitchOut
  (bind _returnvalue (Rendering|Material|CreateDynamicMaterialInstance "/Game/Glitch/M_GlitchEffect.M_GlitchEffect" "None" "None" :!class /Script/Engine.KismetMaterialLibrary))
  (bind _output_get (Variables|Default|SetGlitchMaterialInstance _returnvalue))
  (Rendering|AddorUpdateBlendable (Variables|Default|GetPostProcess) _output_get 1.0 :!class /Script/Engine.PostProcessComponent)
  (bind _fadevalue (Timeline|타임라인_1 PlayFromStart)
    (:Update
      (Rendering|Material|SetScalarParameterValue _output_get "GlitchStrength" _fadevalue :!class /Script/Engine.MaterialInstanceDynamic))))

(event Custom|Glitch
  ;[0.15 0.15 0.15 0.5] Glitch
  (bind _returnvalue (Rendering|Material|CreateDynamicMaterialInstance "/Game/Glitch/M_GlitchEffect.M_GlitchEffect" "None" "None" :!class /Script/Engine.KismetMaterialLibrary))
  (bind _output_get (Variables|Default|SetGlitchMaterialInstance _returnvalue))
  (Rendering|AddorUpdateBlendable (Variables|Default|GetPostProcess) _output_get 1.0 :!class /Script/Engine.PostProcessComponent)
  (bind _fadevalue (Timeline|타임라인 PlayFromStart)
    (:Update
      (Rendering|Material|SetScalarParameterValue _output_get "GlitchStrength" _fadevalue :!class /Script/Engine.MaterialInstanceDynamic))))

(event Custom|HitGlitch
  ;[0.15 0.15 0.15 0.5] HitGlitch
  (CameraFades|StartCameraFade (Variables|/Script/Engine.PlayerController|GetPlayerCameraManager (Game|GetPlayerController 0)) 0.1 0.0 1.0 "(R=1.000000,G=0.000000,B=0.000000,A=1.000000)" false false)
  (bind _returnvalue (Rendering|Material|CreateDynamicMaterialInstance "/Game/Glitch/M_GlitchEffect.M_GlitchEffect" "None" "None" :!class /Script/Engine.KismetMaterialLibrary))
  (bind _output_get (Variables|Default|SetGlitchMaterialInstance _returnvalue))
  (Rendering|AddorUpdateBlendable (Variables|Default|GetPostProcess) _output_get 1.0 :!class /Script/Engine.PostProcessComponent)
  (bind _fadevalue (Timeline|타임라인_0 PlayFromStart)
    (:Update
      (Rendering|Material|SetScalarParameterValue _output_get "GlitchStrength" _fadevalue :!class /Script/Engine.MaterialInstanceDynamic))))

(fn ConstructionScript)