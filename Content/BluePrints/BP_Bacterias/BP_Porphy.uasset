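; BP_Porphy is a bacteria actor that takes hits from overlapping Bullet or Pistol tagged actors, protected by a one-hit shield.
; Capsule overlaps destroy bullets, then either break the shield and hide its mesh, or call TakeDamageBac once the shield is gone.
; A short timer after the shield breaks ignores further hits, so the breaking shot does not also deal damage.
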(event OnComponentBeginOverlap(Capsule)
  (params (OverlappedComponent :type Primitive%20Component%20Object%20Reference) (OtherActor :type Actor%20Object%20Reference) (OtherComp :type Primitive%20Component%20Object%20Reference) (OtherBodyIndex :type Integer) (bFromSweep :type Boolean) (SweepResult :type Hit%20Result%20Structure%20%28by%20ref%29))
  (if (Actor|ActorHasTag OtherActor "Bullet")
    (Actor|DestroyActor OtherActor)
    (if (not (Variables|Default|GetbShieldHitRecently)) :!label _label
      (if (Variables|Default|GetShield)
        (Variables|Default|SetShield false)
        (Variables|Default|SetbShieldHitRecently true)
        (Development|SetHiddeninGame (Variables|Default|GetShieldMesh) true false)
        (Utilities|Time|SetTimerbyEvent (delegate Custom|false) 0.2)
        (Development|PrintString "ShieldHit")
        (else
          (Development|PrintString "Hit")
          (Class|BacteriaBase|TakeDamageBac))))
    (elif (Actor|ActorHasTag OtherActor "Pistol")
      (goto _label))))

(event Custom|false
  (Variables|Default|SetbShieldHitRecently false))

(fn ConstructionScript)