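; BP_ToothRoot is a VR puzzle actor that previews and enables tooth head attachment when the player looks at it.
; It caches the BP_PuzzleVRPawn on BeginPlay, then each Tick until completed compares the camera's forward vector with the direction to its Sphere using a dot product threshold.
; When highlighting is allowed and the gaze is close enough, it shows ToothHead and sets AbleAttach; otherwise it clears both.
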(event EventBeginPlay
  (bind _asbp_puzzle_vrpawn (Utilities|Casting|CastToBP_PuzzleVRPawn (Game|Player|GetPlayerPawn 0)))
  (Variables|Default|SetPlayerPawn _asbp_puzzle_vrpawn))

(event EventTick
  (params (DeltaSeconds :type Float%20%28single-precision%29))
  (bind _toothhead (Variables|Default|GetToothHead))
  (bind _playerpawn (Variables|Default|GetPlayerPawn))
  (bind _camera (Variables|/Game/BluePrints/PuzzleLevel/BP_PuzzleVRPawn.BP_PuzzleVRPawn_C|GetCamera _playerpawn))
  (if (not (Variables|Default|GetbCompleted))
    (if (and (Variables|Default|GetbCanHighLight) (> (Math|Vector|DotProduct (Math|Vector|Normalize (- (Transformation|GetWorldLocation (Variables|Default|GetSphere)) (Transformation|GetWorldLocation _camera))) (Math|Vector|GetForwardVector _camera)) 0.93))
      (Variables|Default|SetbAbleAttach true)
      (Development|SetHiddeninGame _toothhead false false)
      (else
        (Variables|Default|SetbAbleAttach false)
        (Development|SetHiddeninGame _toothhead true false)))))

(fn ConstructionScript)