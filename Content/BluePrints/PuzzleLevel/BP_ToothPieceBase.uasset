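; Base VR puzzle piece for assembling a tooth from grabbable fragments and fitting it onto a root.
; An overlapping piece within rotation tolerance triggers haptics and snaps on when dropped, merging both groups' shared piece arrays.
; Grabbing any piece reparents its group to it.
; At six pieces, an emissive timeline masks the swap to the complete mesh, which completes ToothRoot when dropped on it.
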(event OnComponentBeginOverlap(Sphere)
  (params (OverlappedComponent :type Primitive%20Component%20Object%20Reference) (OtherActor :type Actor%20Object%20Reference) (OtherComp :type Primitive%20Component%20Object%20Reference) (OtherBodyIndex :type Integer) (bFromSweep :type Boolean) (SweepResult :type Hit%20Result%20Structure%20%28by%20ref%29))
  ;[0.15 0.15 0.15 0.5] AbleAttach
  (bind _asbp_tooth_piece_base (Utilities|Casting|CastToBP_ToothPieceBase OtherActor))
  (bind _output_get (Variables|Default|SetOtherToothPiece _asbp_tooth_piece_base))
  (Variables|Default|SetbOverlapping true)
  (Development|PrintString (Utilities|String|Append "overlap: " (Utilities|GetDisplayName _output_get)) false))

(event OnComponentEndOverlap(Sphere)
  (params (OverlappedComponent :type Primitive%20Component%20Object%20Reference) (OtherActor :type Actor%20Object%20Reference) (OtherComp :type Primitive%20Component%20Object%20Reference) (OtherBodyIndex :type Integer))
  ;[0.15 0.15 0.15 0.5] AbleAttach
  (Variables|Default|SetbOverlapping false)
  (Development|PrintString "overlap end" false))

(event OnGrabbed(GrabComponent)
  ;[0.15 0.15 0.15 0.5] OnGrabbed
  (if (Variables|Default|GetbAbleRootAttach)
    (Variables|/Game/BluePrints/PuzzleLevel/BP_ToothRoot.BP_ToothRoot_C|SetbCanHighLight (Variables|Default|GetToothRoot) true)
    (else
      (Collision|SetCollisionEnabled (Variables|컴포넌트|GetSphere) "QueryOnly")
      (for _array_element (Variables|Default|GetAttachedPieceArray)
        (Development|PrintString (Utilities|String|Append "Reattach: " (Utilities|GetDisplayName _array_element)) false)
        (if (!= _array_element self)
          (Transformation|AttachComponentToComponent (Variables|BP_ToothPieceBase_C|GetToothCell _array_element) (Variables|컴포넌트|GetToothCell) "None" "SnapToTarget" "SnapToTarget" "KeepWorld" true)
          (Collision|SetCollisionEnabled (Variables|BP_ToothPieceBase_C|GetToothCell _array_element) "NoCollision")
          (Collision|SetCollisionEnabled (Variables|BP_ToothPieceBase_C|GetSphere _array_element) "NoCollision")
          (Development|PrintString (Utilities|String|Append "[NoCollision] " (Utilities|GetDisplayName _array_element)) false)))
      (CallFunction|Debug))))

(event OnDropped(GrabComponent)
  (bind _toothcell (Variables|컴포넌트|GetToothCell))
  (bind _toothroot (Variables|Default|GetToothRoot))
  (bind _returnvalue (Transformation|GetWorldTransform _toothcell))
  ;[0.15 0.15 0.15 0.5] OnDropped
  (if (Variables|Default|GetbAbleRootAttach)
    (if (Variables|/Game/BluePrints/PuzzleLevel/BP_ToothRoot.BP_ToothRoot_C|GetbAbleAttach _toothroot)
      (Niagara|SpawnSystematLocation "/Game/Niagara/NS_Cloud.NS_Cloud" (.location _returnvalue) (.rotation _returnvalue) (.scale _returnvalue))
      (Actor|DestroyActor)
      (Rendering|Material|SetMaterial (Variables|/Game/BluePrints/PuzzleLevel/BP_ToothRoot.BP_ToothRoot_C|GetToothHead _toothroot) 0 "/Game/Asset/denture/dente.dente")
      (Variables|/Game/BluePrints/PuzzleLevel/BP_ToothRoot.BP_ToothRoot_C|SetbCompleted _toothroot true)
      (else
        (Variables|/Game/BluePrints/PuzzleLevel/BP_ToothRoot.BP_ToothRoot_C|SetbCanHighLight _toothroot false)))
    (else
      (Development|PrintString (Utilities|String|Append "Dropped: " (Utilities|GetDisplayName self)) false)
      (if (Variables|Default|GetbAbleAttach)
        (CallFunction|Attach)
        (Collision|SetCollisionEnabled (Variables|컴포넌트|GetToothCell) "NoCollision")
        (else
          (for _array_element (Variables|Default|GetAttachedPieceArray)
            (Collision|SetCollisionEnabled (Variables|BP_ToothPieceBase_C|GetToothCell _array_element) "QueryAndPhysics")
            (Development|PrintString (Utilities|String|Append "[CollisionEnabled] " (Utilities|GetDisplayName _array_element)) false)))))))

(event Custom|Attach
  (bind _toothcell (Variables|컴포넌트|GetToothCell))
  ;[0.15 0.15 0.15 0.5] AttachComponentToComponent
  (Audio|PlaySoundatLocation "/Game/Sound/sharp-clap-329723.sharp-clap-329723" (Transformation|GetWorldLocation _toothcell) "0, 0, 0" 1.0 1.0 0.0 0 0 0 0)
  (Transformation|AttachComponentToComponent _toothcell (Variables|BP_ToothPieceBase_C|GetToothCell (Variables|Default|GetOtherToothPiece)) "None" "SnapToTarget" "SnapToTarget" "KeepWorld" true)
  (Collision|SetCollisionEnabled (Variables|컴포넌트|GetSphere) "NoCollision")
  (Variables|Default|SetTempArray (Variables|Default|GetAttachedPieceArray))
  (for _array_element (Variables|BP_ToothPieceBase_C|GetAttachedPieceArray (Variables|Default|GetOtherToothPiece))
    (Utilities|Array|AddUnique (Variables|Default|GetTempArray) _array_element))
  (for _array_element_2 (Variables|Default|GetTempArray)
    (bind _output_get (Variables|BP_ToothPieceBase_C|SetAttachedPieceArray _array_element_2 (Variables|Default|GetTempArray))))
  (Development|PrintString (Utilities|String|Append "Attachto: " (Utilities|GetDisplayName (Variables|Default|GetOtherToothPiece))) false)
  (if (>= (Utilities|Array|Length _output_get) 6)
    (CallFunction|Clear (Variables|Default|GetOtherToothPiece))))

(event Custom|Debug
  ;[0.15 0.15 0.15 0.5] OnGrabbed
  (Development|PrintString (Utilities|String|Append "Grabbed: AbleAttach(" (Utilities|String|ToString(Boolean) (Variables|Default|GetbAbleAttach)) ") / Overlapping(" (Utilities|String|ToString(Boolean) (Variables|Default|GetbOverlapping)) ") / SphereCollision(" (Utilities|String|EnumtoString (Collision|GetCollisionEnabled (Variables|컴포넌트|GetSphere)))) false))

(event Custom|Clear
  (bind _puzzlemanager (Variables|Default|GetPuzzleManager))
  (bind _toothcell (Variables|컴포넌트|GetToothCell))
  (Development|PrintString "Clear" false)
  (bind _이머시브 (Timeline|타임라인 Play)
    (:Update
      (Rendering|Material|SetScalarParameterValue (Variables|Default|GetDynamicMat) "DenteEmissive" _이머시브 :!class /Script/Engine.MaterialInstanceDynamic))
    (:Finished
      (if (Variables|Default|GetbIsReverse)
        (Variables|Default|SetbAbleRootAttach true)
        (else
          (Components|StaticMesh|SetStaticMesh _toothcell (Variables|/Game/BluePrints/PuzzleLevel/BP_PuzzleManager.BP_PuzzleManager_C|GetCompletePiece _puzzlemanager))
          (Rendering|Material|SetMaterial _toothcell 0 (Variables|Default|GetDynamicMat))
          (for _array_element (Variables|/Game/BluePrints/PuzzleLevel/BP_PuzzleManager.BP_PuzzleManager_C|GetToothPieceArray _puzzlemanager)
            (if (!= _array_element self)
              (Actor|DestroyActor _array_element)))
          (Variables|Default|SetbIsReverse true)
          (Timeline|타임라인 ReverseFromEnd))))))

(event EventBeginPlay
  ;[0.15 0.15 0.15 0.5] BeginPlay
  (Utilities|FlowControl|Delay 0.1)
  (Utilities|Array|Add (Variables|Default|GetAttachedPieceArray) self)
  (Rendering|Material|SetMaterial (Variables|컴포넌트|GetToothCell) 0 (Variables|Default|GetDynamicMat)))

(event EventTick
  (params (DeltaSeconds :type Float%20%28single-precision%29))
  (bind _grabcomponent (Variables|Default|GetGrabComponent))
  (bind _othertoothpiece (Variables|Default|GetOtherToothPiece))
  (bind _returnvalue (Transformation|GetWorldRotation _grabcomponent))
  (bind _grabcomponent_2 (Variables|BP_ToothPieceBase_C|GetGrabComponent _othertoothpiece))
  (bind _returnvalue_2 (Transformation|GetWorldRotation _grabcomponent_2))
  (bind (_roll _pitch _yaw) (Math|Rotator|BreakRotator _returnvalue))
  (bind (_roll_2 _pitch_2 _yaw_2) (Math|Rotator|BreakRotator _returnvalue_2))
  ;[0.15 0.15 0.15 0.5] AbleAttach
  (if (Variables|Default|GetbOverlapping)
    (if (Math|Boolean|ANDBoolean (<= (Math|Float|Absolute(Float) (- _roll_2 _roll)) 15.0) (<= (Math|Float|Absolute(Float) (- _pitch_2 _pitch)) 15.0) (<= (Math|Float|Absolute(Float) (- _yaw_2 _yaw)) 15.0))
      (Variables|Default|SetbAbleAttach true)
      (Development|PrintString "AbleAttach" false)
      (Class|PlayerController|PlayHapticEffect (Game|GetPlayerController 0) "/Game/VRTemplate/Haptics/PistolFireHapticEffect.PistolFireHapticEffect" (Default|GetHeldbyHand (Variables|Default|GetGrabComponent)) 1.0 false)
      (else
        (Variables|Default|SetbAbleAttach false :!label _label)))
    (else
      (goto _label))))

(fn ConstructionScript)