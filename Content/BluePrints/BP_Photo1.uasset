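; BP_Photo1 is an actor that plays a one-shot slideshow of four photo components when play begins.
; BeginPlay zeroes every photo's scale, then a chain of timelines scales up one photo at a time.
; Each timeline's finish waits briefly, hides that photo and starts the next, until the last one is hidden.
; Tick and overlap events are empty, and a cast to VR_EndingPlayerPawn is never run.
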(event EventBeginPlay
  (Transformation|SetWorldScale3D (Variables|Default|Getphoto1) "0, 0, 0")
  (bind _scalevalue (Timeline|AppearTimeline Play)
    (:Update
      (Transformation|SetWorldScale3D (Variables|Default|Getphoto1) (Math|Conversions|ToVector(Float) _scalevalue)))
    (:Finished
      (Utilities|FlowControl|Delay 2.0)
      (Rendering|SetVisibility (Variables|Default|Getphoto1) false false)
      (bind _scalevalue_2 (Timeline|타임라인 Play)
        (:Update
          (Transformation|SetWorldScale3D (Variables|Default|Getphoto2) (Math|Conversions|ToVector(Float) _scalevalue_2)))
        (:Finished
          (Utilities|FlowControl|Delay 2.0)
          (Rendering|SetVisibility (Variables|Default|Getphoto2) false false)
          (bind _scalevalue_3 (Timeline|타임라인_0 Play)
            (:Update
              (Transformation|SetWorldScale3D (Variables|Default|Getphoto3) (Math|Conversions|ToVector(Float) _scalevalue_3)))
            (:Finished
              (Utilities|FlowControl|Delay 2.0)
              (Rendering|SetVisibility (Variables|Default|Getphoto3) false false)
              (bind _scalevalue_4 (Timeline|타임라인_1 Play)
                (:Update
                  (Transformation|SetWorldScale3D (Variables|Default|Getphoto4) (Math|Conversions|ToVector(Float) _scalevalue_4)))
                (:Finished
                  (Utilities|FlowControl|Delay 2.0)
                  (Rendering|SetVisibility (Variables|Default|Getphoto4) false false))))))))))

(event EventTick
  (params (DeltaSeconds :type Float%20%28single-precision%29)))

(event Collision|EventActorBeginOverlap
  (params (OtherActor :type Actor%20Object%20Reference)))

(fn ConstructionScript)