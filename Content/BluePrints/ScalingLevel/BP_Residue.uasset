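; BP_Residue is a residue actor in the scaling level that the player shrinks with a water gun.
; On BeginPlay it randomly either destroys itself or takes a random rotation, scale and material and adds to the ScalingManager's total count.
; While a WaterGun1 overlaps it, Tick shrinks it gradually until a minimum scale, then swaps it for a BP_GrabResidue carrying the same material and manager.
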(event OnComponentBeginOverlap(Residue)
  (params (OverlappedComponent :type Primitive%20Component%20Object%20Reference) (OtherActor :type Actor%20Object%20Reference) (OtherComp :type Primitive%20Component%20Object%20Reference) (OtherBodyIndex :type Integer) (bFromSweep :type Boolean) (SweepResult :type Hit%20Result%20Structure%20%28by%20ref%29))
  (Utilities|Casting|CastToWaterGun1 OtherActor)
  (if true
    (Variables|Default|SetbOverlapped true)
    (Development|PrintString "residue Overlap ON")))

(event OnComponentEndOverlap(Residue)
  (params (OverlappedComponent :type Primitive%20Component%20Object%20Reference) (OtherActor :type Actor%20Object%20Reference) (OtherComp :type Primitive%20Component%20Object%20Reference) (OtherBodyIndex :type Integer))
  (Utilities|Casting|CastToWaterGun1 OtherActor)
  (if true
    (Variables|Default|SetbOverlapped false)))

(event Custom|SpawnActor
  (bind _returnvalue (Game|SpawnActorfromClass "/Game/BluePrints/ScalingLevel/BP_GrabResidue.BP_GrabResidue_C" (Transformation|GetActorTransform) "Undefined" "MultiplyWithRoot" 0 0))
  (Variables|/Game/BluePrints/ScalingLevel/BP_GrabResidue.BP_GrabResidue_C|SetScalingManager _returnvalue (Variables|Default|GetScalingManager))
  (Rendering|Material|SetMaterial (Variables|/Game/BluePrints/ScalingLevel/BP_GrabResidue.BP_GrabResidue_C|GetResidue _returnvalue) 0 (Rendering|Material|GetMaterial (Variables|Default|GetResidue) 0))
  (Actor|DestroyActor))

(event EventBeginPlay
  (bind _residue (Variables|Default|GetResidue))
  (bind _scalingmanager (Variables|Default|GetScalingManager))
  (if (Math|Random|RandomBool)
    (Transformation|SetWorldRotation _residue (Math|Random|RandomRotator true) false false)
    (bind _output_get (Variables|Default|SetScale (Math|Random|RandomFloatinRange 0.3 0.7)))
    (Transformation|SetWorldScale3D _residue (Math|Vector|MakeVector _output_get _output_get _output_get))
    (Rendering|Material|SetMaterial _residue 0 (.OutItem (Utilities|Array|Random (Variables|Default|GetMaterials))))
    (Variables|/Game/BluePrints/BP_ScalingManager.BP_ScalingManager_C|SetTotalCount _scalingmanager (+ (Variables|/Game/BluePrints/BP_ScalingManager.BP_ScalingManager_C|GetTotalCount _scalingmanager) 1.0))
    (else
      (Actor|DestroyActor))))

(event EventTick
  (params (DeltaSeconds :type Float%20%28single-precision%29))
  (Utilities|FlowControl|Sequence
    (:then_0
      (if (and (Variables|Default|GetbOverlapped) (> (Variables|Default|GetScale) 0.3))
        (bind _output_get (Variables|Default|SetScale (- (Variables|Default|GetScale) 0.001)))
        (Transformation|SetWorldScale3D (Variables|Default|GetResidue) (Math|Vector|MakeVector _output_get _output_get _output_get))
        (Development|PrintString "reduce")
        (if (<= (Variables|Default|GetScale) 0.3)
          (CallFunction|SpawnActor))))))

(fn ConstructionScript)