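; Base tooth actor for a scaling level, where teeth are cleaned while overlapped by a WaterGun1.
; Each tooth registers with a Manager and starts with random dirt, shown through a material layer opacity parameter.
; Tick lowers the dirt during overlap, notifying the Manager once when clean.
; At full Manager progress, an overlapped tooth awards reputation, updates stage state, triggers BP_Glitch and opens SittingRoom after a delay.
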(event OnComponentBeginOverlap(StaticMesh)
  (params (OverlappedComponent :type Primitive%20Component%20Object%20Reference) (OtherActor :type Actor%20Object%20Reference) (OtherComp :type Primitive%20Component%20Object%20Reference) (OtherBodyIndex :type Integer) (bFromSweep :type Boolean) (SweepResult :type Hit%20Result%20Structure%20%28by%20ref%29))
  (Utilities|Casting|CastToWaterGun1 OtherActor)
  (if true
    (Variables|Default|SetbOverlapped true)
    (Development|PrintString "Overlap ON" false)))

(event OnComponentEndOverlap(StaticMesh)
  (params (OverlappedComponent :type Primitive%20Component%20Object%20Reference) (OtherActor :type Actor%20Object%20Reference) (OtherComp :type Primitive%20Component%20Object%20Reference) (OtherBodyIndex :type Integer))
  (Utilities|Casting|CastToWaterGun1 OtherActor)
  (if true
    (Variables|Default|SetbOverlapped false)))

(event EventBeginPlay
  (bind _manager (Variables|Default|GetManager))
  (bind _returnvalue (Rendering|Material|CreateDynamicMaterialInstance (Variables|Default|GetStaticMesh) 0 0 "None" :!class /Script/Engine.PrimitiveComponent))
  (Variables|Default|SetDynamicMat _returnvalue)
  (CallFunction|SetScalarOpacity (Math|Random|RandomFloatinRange 0.5 1.1))
  (Variables|/Game/BluePrints/BP_ScalingManager.BP_ScalingManager_C|SetTotalCount _manager (+ (Variables|/Game/BluePrints/BP_ScalingManager.BP_ScalingManager_C|GetTotalCount _manager) 1.0))
  (bind _outactors (Actor|GetAllActorsOfClass "/Game/BluePrints/BP_Glitch.BP_Glitch_C"))
  (Variables|Default|SetBP%20Glitch (Utilities|Array|Get(acopy) _outactors)))

(event EventTick
  (params (DeltaSeconds :type Float%20%28single-precision%29))
  (if (Variables|Default|GetbOverlapped)
    (CallFunction|CleanTooth)
    (if (== (Variables|/Game/BluePrints/BP_ScalingManager.BP_ScalingManager_C|GetCleanProgress (Variables|Default|GetManager)) 1e+02)
      (Utilities|FlowControl|DoOnce false
        (:Completed
          (bind _asbp_game_instance (Utilities|Casting|CastToBP_GameInstance (Game|GetGameInstance)))
          (Variables|/Game/BluePrints/BP_GameInstance.BP_GameInstance_C|SetReputation _asbp_game_instance (+ (Variables|/Game/BluePrints/BP_GameInstance.BP_GameInstance_C|GetReputation _asbp_game_instance) 25.0))
          (Utilities|Array|SetArrayElem (Variables|/Game/BluePrints/BP_GameInstance.BP_GameInstance_C|GetStageClear? _asbp_game_instance) 0 true)
          (Variables|/Game/BluePrints/BP_GameInstance.BP_GameInstance_C|SetCurrent_Stage _asbp_game_instance 0)
          (Default|Glitch (Variables|Default|GetBP%20Glitch))
          (Utilities|FlowControl|Delay 2.0)
          (Game|OpenLevel(byName) "SittingRoom"))))))

(fn ConstructionScript)

(fn CleanTooth
  (bind _dirtypoint (Variables|Default|GetDirtyPoint))
  (bind _returnvalue (- _dirtypoint 0.005))
  (if (< _returnvalue 0.0)
    (if (not (Variables|Default|GetbUpdateCB))
      (Variables|Default|SetbUpdateCB true)
      (Default|UpdateCB (Variables|Default|GetManager)))
    (else
      (CallFunction|SetScalarOpacity _returnvalue))))

(fn SetScalarOpacity
  (params (DirtyPoint :type Float%20%28double-precision%29))
  (bind _output_get (Variables|Default|SetDirtyPoint DirtyPoint))
  (Rendering|Material|SetScalarParameterValuebyInfo (Variables|Default|GetDynamicMat) (Utilities|Struct|MakeMaterialParameterInfo "ScalarOpacity" "LayerParameter" 1) _output_get))