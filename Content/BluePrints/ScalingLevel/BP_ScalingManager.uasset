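; BP_ScalingManager tracks cleaning progress in the VR tooth-scaling level and handles stage completion.
; UpdateCB increments progress and refreshes the pawn's Cleaned_bar widget; on completion it updates GameInstance reputation and stage state, plays a sound, glitches, fades, and opens SittingRoom.
; NotifyToothCleaned is a separate bar-update path, with an inverted ratio (total/cleaned).
; RegisterTooth is empty, and the dirty-tooth counting and BP_Glitch lookup nodes are unwired.
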(event Custom|UpdateCB
  (bind _asvr_scaling_player_pawn (Utilities|Casting|CastToVR_ScalingPlayerPawn (Game|Player|GetPlayerPawn 0)))
  (bind _ascleaned_bar (Utilities|Casting|CastToCleaned_bar (UserInterface|GetUserWidgetObject (Variables|/Game/BluePrints/ScalingLevel/VR_ScalingPlayerPawn.VR_ScalingPlayerPawn_C|GetCleanedBar _asvr_scaling_player_pawn))))
  (bind _output_get (Variables|Default|SetCleanProgress (+ 1.0 (Variables|Default|GetCleanProgress))))
  (Default|UpdateHP _ascleaned_bar (/ _output_get (Variables|Default|GetTotalCount)))
  (Development|PrintString "Update" false)
  (if (>= (/ _output_get (Variables|Default|GetTotalCount)) 1.0)
    (bind _asbp_game_instance (Utilities|Casting|CastToBP_GameInstance (Game|GetGameInstance)))
    (Variables|/Game/BluePrints/BP_GameInstance.BP_GameInstance_C|SetReputation _asbp_game_instance (+ (Variables|/Game/BluePrints/BP_GameInstance.BP_GameInstance_C|GetReputation _asbp_game_instance) 2e+01))
    (Utilities|Array|SetArrayElem (Variables|/Game/BluePrints/BP_GameInstance.BP_GameInstance_C|GetStageClear? _asbp_game_instance) 0 true)
    (Variables|/Game/BluePrints/BP_GameInstance.BP_GameInstance_C|SetCurrent_Stage _asbp_game_instance 0)
    (Utilities|FlowControl|Delay 1.0)
    (Audio|PlaySoundatLocation "/Game/Sound/clear-notification-355970.clear-notification-355970" "0, 0, 0" "0, 0, 0" 1.0 1.0 0.0 0 0 0 0)
    (Utilities|FlowControl|Delay 1.0)
    (Default|Glitch (Variables|Default|GetBPGlitch))
    (CallFunction|FadeOut)
    (Utilities|FlowControl|Delay 2.0)
    (Game|OpenLevel(byName) "SittingRoom")))

(event Custom|FadeOut
  (CameraFades|StartCameraFade :self (Variables|/Script/Engine.PlayerController|GetPlayerCameraManager (Game|GetPlayerController 0)) :ToAlpha 1.0 :Duration 2.0 :bHoldWhenFinished true))

(event EventBeginPlay
  (bind _ascleaned_bar (Utilities|Casting|CastToCleaned_bar (UserInterface|GetUserWidgetObject (Variables|/Game/BluePrints/ScalingLevel/VR_ScalingPlayerPawn.VR_ScalingPlayerPawn_C|GetCleanedBar (Variables|Default|GetPlayer)))))
  (Variables|Default|SetCleanedBar _ascleaned_bar))

(fn ConstructionScript)

(fn RegisterTooth
  (params (Tooth :type BP%20Tooth%20Base%20Object%20Reference)))

(fn NotifyToothCleaned
  (params (Tooth :type BP%20Tooth%20Base%20Object%20Reference))
  (bind _cleanedbarref (Variables|Default|GetCleanedBarRef))
  (bind _output_get (Variables|Default|SetCleanedCount (+ (Variables|Default|GetCleanedCount) 1)))
  (Default|UpdateHP _cleanedbarref (Math|Float|Clamp(Float) (/ (Variables|Default|GetTotalCount) _output_get)))
  (Progress|SetPercent (Variables|/Game/UI/Widgets/Stage/Cleaned_bar.Cleaned_bar_C|GetProgress_Cleaning _cleanedbarref) (Math|Float|Clamp(Float) (/ (Variables|Default|GetTotalCount) _output_get))))