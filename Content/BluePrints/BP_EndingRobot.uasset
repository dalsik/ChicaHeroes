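; BP_EndingRobot is a grabbable robot actor that triggers the ending text.
; When its GrabComponent fires OnGrabbed, it creates an EndingText widget for the first player controller and adds it to the viewport.
; Unconnected leftover logic would, after a delay, use a timeline to interpolate the robot's rotation and slide it along negative X, but it never runs.
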(event OnGrabbed(GrabComponent)
  (bind _returnvalue (UserInterface|CreateWidget "/Game/BluePrints/Story/EndingText.EndingText_C" (Game|GetPlayerController 0)))
  (UserInterface|Viewport|AddtoViewport _returnvalue 0))

(event EventBeginPlay)

(fn ConstructionScript)