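; BP_Tutorial is a VR widget actor, apparently a tutorial menu derived from the main menu.
; Left and right menu Interact inputs press and release the pointer key on VRPawnSittingRoom's widget interaction components.
; A custom event destroys the actor.
; Setup (mapping context, level-selector delete binding) and RotateMainMenu's smoothed camera-follow exist but are disconnected, leaving BeginPlay and Tick empty.
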(event Custom|DeleteWidget_이벤트
  (Actor|DestroyActor))

(event Input|EnhancedActionEvents|EnhancedInputActionIA_Menu_Interact_Left_Pressed
  (params (ActionValue :type Boolean) (ElapsedSeconds :type Float%20%28double-precision%29) (TriggeredSeconds :type Float%20%28double-precision%29) (InputAction :type Input%20Action%20Object%20Reference :default "/Game/VRTemplate/Input/Actions/IA_Menu_Interact_Left_Pressed.IA_Menu_Interact_Left_Pressed"))
  (bind _vrpawnsittingroom (Variables|Default|GetVRPawnSittingRoom))
  (bind _widgetinteractionleft (Variables|/Game/GameProject_Player/VRPawn_SittingRoom.VRPawn_SittingRoom_C|GetWidgetInteractionLeft _vrpawnsittingroom))
  (:Started
    (Class|WidgetInteractionComponent|PressPointerKey _widgetinteractionleft "LeftMouseButton"))
  (:Canceled
    (Class|WidgetInteractionComponent|ReleasePointerKey _widgetinteractionleft "LeftMouseButton" :!label _label))
  (:Completed
    (goto _label)))

(event Input|EnhancedActionEvents|EnhancedInputActionIA_Menu_Interact_Right_Pressed
  (params (ActionValue :type Boolean) (ElapsedSeconds :type Float%20%28double-precision%29) (TriggeredSeconds :type Float%20%28double-precision%29) (InputAction :type Input%20Action%20Object%20Reference :default "/Game/VRTemplate/Input/Actions/IA_Menu_Interact_Right_Pressed.IA_Menu_Interact_Right_Pressed"))
  (bind _vrpawnsittingroom (Variables|Default|GetVRPawnSittingRoom))
  (bind _widgetinteractionright (Variables|/Game/GameProject_Player/VRPawn_SittingRoom.VRPawn_SittingRoom_C|GetWidgetInteractionRight _vrpawnsittingroom))
  (:Started
    (Class|WidgetInteractionComponent|PressPointerKey _widgetinteractionright "LeftMouseButton"))
  (:Canceled
    (Class|WidgetInteractionComponent|ReleasePointerKey _widgetinteractionright "LeftMouseButton" :!label _label))
  (:Completed
    (goto _label)))

(event EventBeginPlay)

(event Collision|EventActorBeginOverlap
  (params (OtherActor :type Actor%20Object%20Reference)))

(event EventTick
  (params (DeltaSeconds :type Float%20%28single-precision%29)))

(fn ConstructionScript)

(fn RotateMainMenu
  (params (DeltaTime :type Float%20%28double-precision%29))
  (bind _returnvalue (Game|GetPlayerCameraManager 0))
  (bind _defaultsceneroot (Variables|Default|GetDefaultSceneRoot))
  (bind _transformcomponent (Variables|/Script/Engine.PlayerCameraManager|GetTransformComponent _returnvalue))
  (Transformation|SetActorTransform (Math|Transform|MakeTransform (Math|Interpolation|VInterpTo (Transformation|GetWorldLocation _defaultsceneroot) (Transformation|GetWorldLocation _transformcomponent) DeltaTime 0.6) (Math|Rotator|MakeRotator 0.0 0.0 (.yaw (Math|Interpolation|RInterpTo (Transformation|GetWorldRotation _defaultsceneroot) (Transformation|GetWorldRotation _transformcomponent) DeltaTime 0.8))) "1.000000,1.000000,1.000000")))