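; BP_spawnCar is a car spawner actor that periodically spawns a random car at its own transform.
; Tick drives a Delay of random 1–12 second length, which ignores re-triggers while pending and so acts as a repeating timer calling SpawnCar.
; SpawnCar picks one of five entries from the Car class array, spawns it, then adds an audio component with spatialization enabled to the new car.
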(event Custom|SpawnCar
  ;[0.15 0.15 0.15 0.5] SpawnCar
  (bind _returnvalue (Game|SpawnActorfromClass (Utilities|Array|Get(acopy) (Variables|Default|GetCar) (Math|Random|RandomIntegerinRange 0 4)) (Transformation|GetActorTransform) "Undefined" "MultiplyWithRoot" 0 0))
  (bind _returnvalue_2 (AddComponent|AddAudioComponent _returnvalue false))
  (Variables|/Script/Engine.AudioComponent|SetbAllowSpatialization _returnvalue_2 true))

(event EventBeginPlay
  (|CallParentFunction) ; 지금 이 노드는 비활성 상태입니다. \n핀을 끌어서 다른 노드를 연결하면 활성화됩니다.
)

(event EventTick
  (params (DeltaSeconds :type Float%20%28single-precision%29))
  (Utilities|FlowControl|Delay (Math|Random|RandomFloatinRange 1.0 12.0))
  (CallFunction|SpawnCar))

(event Collision|EventActorBeginOverlap
  (params (OtherActor :type Actor%20Object%20Reference))
  (|CallParentFunction OtherActor) ; 지금 이 노드는 비활성 상태입니다. \n핀을 끌어서 다른 노드를 연결하면 활성화됩니다.
)

(fn ConstructionScript
  (|CallParentFunction))