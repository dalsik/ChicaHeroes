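; Stage manager for a VR cavity game level, handling enemy setup, player HP and the win or lose outcome.
; BeginPlay shuffles spawn points, gives their teeth a shared dynamic material with Niagara smoke, and picks enemy info.
; Hits update the pawn's HP widget and trigger glitches; clearing stops smoke and animates the tooth material.
; Death, timeout or clear records results in the game instance, stops spawning and fades to SittingRoom.
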(event Custom|FadeOut
  ;[0.15 0.15 0.15 0.5] FadeOut
  (CameraFades|StartCameraFade :self (Variables|/Script/Engine.PlayerController|GetPlayerCameraManager (Game|GetPlayerController 0)) :ToAlpha 1.0 :Duration 0.3 :bHoldWhenFinished true))

(event Custom|GameStop
  ;[0.15 0.15 0.15 0.5] GameStop
  (Class|StageManager|TickDisable)
  (Utilities|Time|ClearTimerbyFunctionName 0 "SpawnTimerHandle"))

(event Custom|FadeIn
  ;[0.15 0.15 0.15 0.5] FadeIn
  (CameraFades|StartCameraFade :self (Variables|/Script/Engine.PlayerController|GetPlayerCameraManager (Game|GetPlayerController 0)) :FromAlpha 1.0 :Duration 2.0))

(event Custom|SceneChange
  ;[0.15 0.15 0.15 0.5] SceneChange
  (Utilities|FlowControl|Sequence
    (:then_0
      (CallFunction|GameStop)
      (Default|GlitchOut (Variables|Default|GetBP_Glitch))
      (Utilities|FlowControl|Delay 0.7)
      (CallFunction|FadeOut)
      (Utilities|FlowControl|Delay 0.3)
      (Game|OpenLevel(byName) "SittingRoom"))
    (:then_1
      (if (Variables|/Game/BluePrints/BP_GameInstance.BP_GameInstance_C|GetbStageCleared (stale EventGameClear _asbp_game_instance))
        (Utilities|FlowControl|DoOnce false
          (:Completed
            (Variables|/Game/BluePrints/BP_GameInstance.BP_GameInstance_C|SetReputation (stale EventGameClear _asbp_game_instance) (+ (Variables|/Game/BluePrints/BP_GameInstance.BP_GameInstance_C|GetReputation (stale EventGameClear _asbp_game_instance)) 2e+01))
            (Utilities|Array|SetArrayElem (Variables|/Game/BluePrints/BP_GameInstance.BP_GameInstance_C|GetStageClear? (stale EventGameClear _asbp_game_instance)) 3 true)
            (Variables|/Game/BluePrints/BP_GameInstance.BP_GameInstance_C|SetCurrent_Stage (stale EventGameClear _asbp_game_instance) 3)))))))

(event Custom|UDHP
  (params (HP%25 :type Float%20%28double-precision%29))
  (bind _asvr_cavity_player_pawn (Utilities|Casting|CastToVR_CavityPlayerPawn (Variables|Default|GetPlayerPawn)))
  (bind _aswbp_healthbar (Utilities|Casting|CastToWBP_healthbar (UserInterface|GetUserWidgetObject (Variables|/Game/BluePrints/StageLevel/VR_CavityPlayerPawn.VR_CavityPlayerPawn_C|GetHPBar _asvr_cavity_player_pawn))))
  (Default|UpdateHP _aswbp_healthbar HP%25))

(event EventBeginPlay
  (bind _spawnpointarray (Variables|Default|GetSpawnPointArray))
  (Utilities|FlowControl|Sequence
    (:then_0
      (Default|Glitch (Variables|Default|GetBP_Glitch))
      (CallFunction|Fadein)
      (Variables|Default|SetPlayerHp (Variables|Default|GetPlayerMaxHP)))
    (:then_1
      (bind _returnvalue (Rendering|Material|CreateDynamicMaterialInstance "/Game/BluePrints/StageLevel/StageLevelMat/M_StageMaster_Inst.M_StageMaster_Inst" "None" "None" :!class /Script/Engine.KismetMaterialLibrary))
      (bind _output_get (Variables|Default|SetDynamicMat _returnvalue))
      (Rendering|Material|SetScalarParameterValuebyInfo _output_get (Utilities|Struct|MakeMaterialParameterInfo "ScalarOpacity" "LayerParameter" 1) 1.0)
      (Utilities|Array|Shuffle _spawnpointarray)
      (for _index (range 0 (Variables|Default|GetSpawnPointNum))
        (Utilities|Array|Add (Variables|Default|GetSpawnPoint) (Transformation|GetWorldLocation (Variables|/Game/BluePrints/StageLevel/BP_SpawnPoint.BP_SpawnPoint_C|GetSpawnPointLocation (Utilities|Array|Get(acopy) _spawnpointarray _index))))
        (Rendering|Material|SetMaterial (Variables|/Game/BluePrints/StageLevel/BP_SpawnPoint.BP_SpawnPoint_C|GetTooth (Utilities|Array|Get(acopy) _spawnpointarray _index)) 0 (Variables|Default|GetDynamicMat))
        (bind _returnvalue_2 (Niagara|SpawnSystematLocation "/Game/Niagara/NS_Smoke.NS_Smoke" (Transformation|GetWorldLocation (Variables|/Game/BluePrints/StageLevel/BP_SpawnPoint.BP_SpawnPoint_C|GetSpawnPointLocation (Utilities|Array|Get(acopy) _spawnpointarray _index))) "0, 0, 0" "1.000000,1.000000,1.000000" false))
        (Utilities|Array|Add (Variables|Default|GetSmokeArray) _returnvalue_2)))
    (:then_2
      (Class|StageManager|PickEnemyInfo)
      (Utilities|Array|Shuffle (Variables|Default|GetEnemy)))))

(event EventMonsterInfo
  (Class|StageManager|PickEnemyInfo)
  (Utilities|Array|Shuffle (Variables|Default|GetEnemy)))

(event EventTimeOver
  (Variables|/Game/BluePrints/BP_GameInstance.BP_GameInstance_C|SetbStageCleared (stale EventGameClear _asbp_game_instance) false)
  (CallFunction|SceneChange))

(event EventOnPlayerAttackedBP
  (params (Damage :type Float%20%28single-precision%29))
  ;[0.15 0.15 0.15 0.5] Hit
  (Audio|PlaySoundatLocation "/Game/Sound/metal-hit-5-193273.metal-hit-5-193273" (Transformation|GetActorLocation (Variables|Default|GetPlayerPawn)) "0, 0, 0" 1.0 1.0 0.0 0 0 0 0)
  (if (not (Variables|Default|GetCastHPBar))
    (bind _asvr_cavity_player_pawn (Utilities|Casting|CastToVR_CavityPlayerPawn (Variables|Default|GetPlayerPawn)))
    (bind _aswbp_healthbar (Utilities|Casting|CastToWBP_healthbar (UserInterface|GetUserWidgetObject (Variables|/Game/BluePrints/StageLevel/VR_CavityPlayerPawn.VR_CavityPlayerPawn_C|GetHPBar _asvr_cavity_player_pawn)))
      (:then
        (Development|PrintString "cast hpbar success")
        (Variables|Default|SetCastHPBar true)
        (bind _output_get (Variables|Default|SetPlayerHp (- (Variables|Default|GetPlayerHp) Damage) :!label _label))
        (Default|UpdateHP _aswbp_healthbar (/ _output_get (Variables|Default|GetPlayerMaxHP)))
        (Default|HitGlitch (Variables|Default|GetBP_Glitch))
        (if (<= (Variables|Default|GetPlayerHp) 0.0)
          (bind _asbp_game_instance (Utilities|Casting|CastToBP_GameInstance (Game|GetGameInstance)))
          (Variables|/Game/BluePrints/BP_GameInstance.BP_GameInstance_C|SetbStageCleared _asbp_game_instance false)
          (CallFunction|SceneChange)))
      (:CastFailed
        (Development|PrintString "cast hpbar fail")))
    (else
      (goto _label))))

(event EventGameClear
  (for _array_element (Variables|Default|GetSmokeArray)
    (Niagara|SetNiagaraVariable(Float) _array_element "User.SpawnRate" 0.0))
  (bind _value (Timeline|타임라인 PlayFromStart)
    (:Update
      (Rendering|Material|SetScalarParameterValuebyInfo (Variables|Default|GetDynamicMat) (Utilities|Struct|MakeMaterialParameterInfo "ScalarOpacity" "LayerParameter" 1) _value)
      (Development|PrintString (Utilities|String|ToString(Float) _value) false))
    (:Finished
      (Audio|PlaySoundatLocation "/Game/Sound/clear-notification-355970.clear-notification-355970" "0, 0, 0" "0, 0, 0" 1.0 1.0 0.0 0 0 0 0)
      (Utilities|FlowControl|Delay 1.0)
      (bind _asbp_game_instance (Utilities|Casting|CastToBP_GameInstance (Game|GetGameInstance)))
      (Variables|/Game/BluePrints/BP_GameInstance.BP_GameInstance_C|SetbStageCleared _asbp_game_instance true)
      (Variables|/Game/BluePrints/BP_GameInstance.BP_GameInstance_C|SetGold _asbp_game_instance (+ (Variables|/Game/BluePrints/BP_GameInstance.BP_GameInstance_C|GetReward _asbp_game_instance) (Variables|/Game/BluePrints/BP_GameInstance.BP_GameInstance_C|GetGold _asbp_game_instance)))
      (CallFunction|SceneChange))))

(fn ConstructionScript)