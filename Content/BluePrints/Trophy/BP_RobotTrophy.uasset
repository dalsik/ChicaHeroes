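; BP_RobotTrophy is a grabbable trophy actor that sends the game to its ending level.
; On BeginPlay it reads the fourth UnlockWeapon flag (index 3) from BP_GameInstance and stays hidden unless that flag is set.
; When its GrabComponent fires OnGrabbed, it starts a camera fade, waits for the fade duration, then opens EndingLevel.
; Only visibility is toggled; the graph does not change collision or grabbability.
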(event OnGrabbed(GrabComponent)
  (bind _returnvalue (Math|Float|MakeLiteralFloat 4.0))
  (CameraFades|StartCameraFade :self (Game|GetPlayerCameraManager 0) :ToAlpha 1.0 :Duration _returnvalue)
  (Utilities|FlowControl|Delay _returnvalue)
  (Game|OpenLevel(byName) "EndingLevel"))

(event EventBeginPlay
  (bind _asbp_game_instance (Utilities|Casting|CastToBP_GameInstance (Game|GetGameInstance)))
  (Rendering|SetActorHiddenInGame (not (Utilities|Array|Get(acopy) (Variables|/Game/BluePrints/BP_GameInstance.BP_GameInstance_C|GetUnlockWeapon _asbp_game_instance) 3))))

(event Collision|EventActorBeginOverlap
  (params (OtherActor :type Actor%20Object%20Reference)))

(event EventTick
  (params (DeltaSeconds :type Float%20%28single-precision%29)))

(fn ConstructionScript)