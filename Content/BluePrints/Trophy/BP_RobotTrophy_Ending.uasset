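; BP_RobotTrophy_Ending is a robot trophy actor, named for the ending, that currently runs no logic.
; BeginPlay and the construction script are empty, leaving the movement graph disconnected.
; That unused graph would, after a delay, play Timeline_FloatUp to lerp location along negative X despite the timeline's name.
; It also blends rotation toward zero through lerped X vectors, with start and target rotation set in another disconnected chain.
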(event EventBeginPlay)

(fn ConstructionScript)