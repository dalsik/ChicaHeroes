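; BP_Photo1 is an ending-level actor that scales four photo components into view when play begins.
; BeginPlay collapses all four to zero scale, then timelines grow each one, with X stretched wider.
; Each timeline's Update, rather than Finished, plays the next, so the four animations start almost together unless their curves stagger them.
; Unconnected leftovers include a VR_EndingPlayerPawn cast and delayed photo hiding.
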(event EventBeginPlay
  (Transformation|SetWorldScale3D (Variables|Default|Getphoto1) "0, 0, 0")
  (bind _scalevalue (Timeline|AppearTimeline Play)
    (:Update
      (Transformation|SetWorldScale3D (Variables|Default|Getphoto1) (Math|Vector|MakeVector (* _scalevalue 1.5) _scalevalue _scalevalue))
      (bind _scalevalue_2 (Timeline|타임라인 Play)
        (:Update
          (Transformation|SetWorldScale3D (Variables|Default|Getphoto2) (Math|Vector|MakeVector (* _scalevalue_2 1.5) _scalevalue_2 _scalevalue_2))
          (bind _scalevalue_3 (Timeline|타임라인_0 Play)
            (:Update
              (Transformation|SetWorldScale3D (Variables|Default|Getphoto3) (Math|Vector|MakeVector (* _scalevalue_3 1.5) _scalevalue_3 _scalevalue_3))
              (bind _scalevalue_4 (Timeline|타임라인_1 Play)
                (:Update
                  (Transformation|SetWorldScale3D (Variables|Default|Getphoto4) (Math|Vector|MakeVector (* _scalevalue_4 1.5) _scalevalue_4 _scalevalue_4)))))))))))

(event EventTick
  (params (DeltaSeconds :type Float%20%28single-precision%29)))

(event Collision|EventActorBeginOverlap
  (params (OtherActor :type Actor%20Object%20Reference)))

(fn ConstructionScript)