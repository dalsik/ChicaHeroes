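; BP_EducationScalingStage is the scaling stage of the VR education level, hosting a tutorial widget that trails the player's view.
; BeginPlay binds the tutorial's end event, caches the VR pawn and adds the menu input mapping.
; Left and right interact inputs drive the pawn's widget interaction pointers as mouse clicks.
; Tick eases position and yaw toward the camera; tutorial end destroys the actor and calls CallDestroyScalingStage.
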(event Custom|End
  (Actor|DestroyActor)
  (Default|CallCallDestroyScalingStage))

(event Input|EnhancedActionEvents|EnhancedInputActionIA_Menu_Interact_Left_Pressed
  (params (ActionValue :type Boolean) (ElapsedSeconds :type Float%20%28double-precision%29) (TriggeredSeconds :type Float%20%28double-precision%29) (InputAction :type Input%20Action%20Object%20Reference :default "/Game/VRTemplate/Input/Actions/IA_Menu_Interact_Left_Pressed.IA_Menu_Interact_Left_Pressed"))
  (bind _as_vrpawn_education_level (Variables|Default|GetAs%20VRPawn%20Education%20Level))
  (bind _widgetinteractionleft (Variables|/Game/GameProject_Player/VRPawn_EducationLevel.VRPawn_EducationLevel_C|GetWidgetInteractionLeft _as_vrpawn_education_level))
  (:Started
    (Class|WidgetInteractionComponent|PressPointerKey _widgetinteractionleft "LeftMouseButton"))
  (:Canceled
    (Class|WidgetInteractionComponent|ReleasePointerKey _widgetinteractionleft "LeftMouseButton" :!label _label))
  (:Completed
    (goto _label)))

(event Input|EnhancedActionEvents|EnhancedInputActionIA_Menu_Interact_Right_Pressed
  (params (ActionValue :type Boolean) (ElapsedSeconds :type Float%20%28double-precision%29) (TriggeredSeconds :type Float%20%28double-precision%29) (InputAction :type Input%20Action%20Object%20Reference :default "/Game/VRTemplate/Input/Actions/IA_Menu_Interact_Right_Pressed.IA_Menu_Interact_Right_Pressed"))
  (bind _as_vrpawn_education_level (Variables|Default|GetAs%20VRPawn%20Education%20Level))
  (bind _widgetinteractionright (Variables|/Game/GameProject_Player/VRPawn_EducationLevel.VRPawn_EducationLevel_C|GetWidgetInteractionRight _as_vrpawn_education_level))
  (:Started
    (Class|WidgetInteractionComponent|PressPointerKey _widgetinteractionright "LeftMouseButton"))
  (:Canceled
    (Class|WidgetInteractionComponent|ReleasePointerKey _widgetinteractionright "LeftMouseButton" :!label _label))
  (:Completed
    (goto _label)))

(event EventBeginPlay
  (bind _returnvalue (Game|GetPlayerController 0))
  (bind _aswb_education_scaling_widget (Utilities|Casting|CastToWB_EducationScalingWidget (UserInterface|GetUserWidgetObject (Variables|Default|GetWidget))))
  (EventDispatchers|BindEventtoCallEnd (Variables|/Game/GameProject_Player/Asset/WB_EducationScalingWidget.WB_EducationScalingWidget_C|GetWB_MainTutorial _aswb_education_scaling_widget) (delegate Custom|End))
  (bind _asvrpawn_education_level (Utilities|Casting|CastToVRPawn_EducationLevel (Game|Player|GetPlayerPawn 0)))
  (bind _output_get (Variables|Default|SetAs%20VRPawn%20Education%20Level _asvrpawn_education_level))
  (Actor|Tick|SetActorTickEnabled _output_get true)
  (Input|EnableInput _returnvalue)
  (Input|AddMappingContext (PlayerController|LocalPlayerSubsystems|GetEnhancedInputLocalPlayerSubsystem _returnvalue) "/Game/VRTemplate/Input/IMC_Menu.IMC_Menu" 1 "(bIgnoreAllPressedKeysUntilRelease=True,bForceImmediately=False,bNotifyUserSettings=False)")
  (Development|PrintString "캐스트 됨"))

(event EventTick
  (params (DeltaSeconds :type Float%20%28single-precision%29))
  (CallFunction|Rotate DeltaSeconds))

(fn ConstructionScript)

(fn Rotate
  (params (Delta :type Float%20%28double-precision%29))
  (bind _returnvalue (Game|GetPlayerCameraManager 0))
  (bind _defaultsceneroot (Variables|Default|GetDefaultSceneRoot))
  (bind _transformcomponent (Variables|/Script/Engine.PlayerCameraManager|GetTransformComponent _returnvalue))
  (Transformation|SetActorTransform (Math|Transform|MakeTransform (Math|Interpolation|VInterpTo (Transformation|GetWorldLocation _defaultsceneroot) (Transformation|GetWorldLocation _transformcomponent) Delta 0.6) (Math|Rotator|MakeRotator 0.0 0.0 (.yaw (Math|Interpolation|RInterpTo (Transformation|GetWorldRotation _defaultsceneroot) (Transformation|GetWorldRotation _transformcomponent) Delta 0.8))) "1.000000,1.000000,1.000000")))