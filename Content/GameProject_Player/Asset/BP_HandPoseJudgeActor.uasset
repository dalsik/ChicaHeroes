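; Hand-pose judge actor for a teeth-themed stage, tracking the player's progress and completing the stage when it is full.
; Each Tick calls CompareHandsAndUpdateProgress, defined outside this graph, and pushes the result to its TeethProgressUI widget.
; At full progress, a DoOnce raises Reputation and records the stage clear in BP_GameInstance.
; It then plays a sound, triggers BP_Glitch after a delay and opens the SittingRoom level.
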(event EventBeginPlay
  (bind _asteeth_progress_ui (Utilities|Casting|CastToTeethProgressUI (UserInterface|GetUserWidgetObject (Variables|Default|GetWidget))))
  (Variables|Default|SetAs%20Teeth%20Progress%20UI _asteeth_progress_ui)
  (bind _asbp_game_instance (Utilities|Casting|CastToBP_GameInstance (Game|GetGameInstance)))
  (Variables|Default|SetAs%20BP%20Game%20Instance _asbp_game_instance)
  (bind _outactors (Actor|GetAllActorsOfClass "/Game/BluePrints/BP_Glitch.BP_Glitch_C"))
  (Variables|Default|SetBP_Glitch (Utilities|Array|Get(acopy) _outactors)))

(event Collision|EventActorBeginOverlap
  (params (OtherActor :type Actor%20Object%20Reference)))

(event EventTick
  (params (DeltaSeconds :type Float%20%28single-precision%29))
  (bind _as_teeth_progress_ui (Variables|Default|GetAs%20Teeth%20Progress%20UI))
  (bind _as_bp_game_instance (Variables|Default|GetAs%20BP%20Game%20Instance))
  (Class|HandPoseJudgeActor|CompareHandsandUpdateProgress)
  (bind _returnvalue (Class|HandPoseJudgeActor|GetProgress))
  (Variables|/Game/GameProject_Player/Asset/TeethProgressUI.TeethProgressUI_C|SetNewProgress _as_teeth_progress_ui _returnvalue)
  (Default|UpdateProgressUI _as_teeth_progress_ui)
  (if (== _returnvalue 1e+02)
    (Utilities|FlowControl|DoOnce false
      (:Completed
        (Variables|/Game/BluePrints/BP_GameInstance.BP_GameInstance_C|SetReputation _as_bp_game_instance (+ (Variables|/Game/BluePrints/BP_GameInstance.BP_GameInstance_C|GetReputation _as_bp_game_instance) 25.0))
        (Utilities|Array|SetArrayElem (Variables|/Game/BluePrints/BP_GameInstance.BP_GameInstance_C|GetStageClear? _as_bp_game_instance) 2 true)
        (Variables|/Game/BluePrints/BP_GameInstance.BP_GameInstance_C|SetCurrent_Stage _as_bp_game_instance 2)
        (Audio|PlaySoundatLocation "/Game/Sound/clear-notification-355970.clear-notification-355970" (Transformation|GetActorLocation (Game|Player|GetPlayerPawn 0)) "0, 0, 0" 1.0 1.0 0.0 0 0 0 0)
        (Utilities|FlowControl|Delay 1.0)
        (Default|Glitch (Variables|Default|GetBP_Glitch))
        (Utilities|FlowControl|Delay 2.0)
        (Game|OpenLevel(byName) "SittingRoom")
        (Class|HandPoseJudgeActor|SetProgress)))))

(fn ConstructionScript)